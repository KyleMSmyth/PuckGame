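; Shared camera for the puck game that frames every BP_PuckGameCharacter found at BeginPlay.
; Each tick it turns toward the players' average location, follows that average's X at a reduced scale and keeps Y fixed.
; It projects players to screen space, rising with accelerating steps while anyone is off screen and sinking toward a minimum height otherwise.
; Code that would add the puck to the tracked actors is disconnected.
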(event EventBeginPlay
  (Utilities|Casting|CastToBP_PuckGameGameMode (Game|GetGameMode))
  (bind _outactors (Actor|GetAllActorsOfClass "/Game/Blueprints/Character/BP_PuckGameCharacter.BP_PuckGameCharacter_C"))
  (bind _output_get (Variables|Default|SetActivePlayers _outactors)))

(event Collision|EventActorBeginOverlap
  (params (OtherActor :type Actor%20Object%20Reference)))

(event EventTick
  (params (DeltaSeconds :type Float%20%28single-precision%29))
  (bind _returnvalue (Transformation|GetActorLocation))
  (bind _returnvalue_2 (Transformation|GetActorLocation))
  (bind _returnvalue_3 (Viewport|GetViewportSize))
  (bind _returnvalue_4 (Viewport|GetViewportSize))
  (bind _self self)
  (bind _collectedplayerlocations (Variables|Default|GetCollectedPlayerLocations))
  (bind _returnvalue_5 (Math|Vector|GetVectorArrayAverage _collectedplayerlocations))
  (bind (_x _y) (Math|Vector2D|BreakVector2D _returnvalue_4))
  (bind (_x_2 _y_2 _z) (Math|Vector|BreakVector _returnvalue))
  (bind (_x_3 _y_3 _z_2) (Math|Vector|BreakVector _returnvalue_2))
  (bind (_x_4 _y_4) (Math|Vector2D|BreakVector2D _returnvalue_3))
  (bind _returnvalue_6 (Transformation|GetActorLocation _self))
  (for (_array_element _array_index) (Variables|Default|GetActivePlayers)
    (Utilities|Array|SetArrayElem _collectedplayerlocations _array_index (Transformation|GetActorLocation _array_element) true)
    (if (Math|Boolean|ANDBoolean (> (.X (Math|Vector2D|BreakVector2D (.ScreenLocation (Class|PlayerController|ProjectWorldLocationtoScreen (Game|GetPlayerController 0) (Transformation|GetActorLocation _array_element) true)))) 0.0) (> (.Y (Math|Vector2D|BreakVector2D (.ScreenLocation (Class|PlayerController|ProjectWorldLocationtoScreen (Game|GetPlayerController 0) (Transformation|GetActorLocation _array_element) true)))) 0.0) (< (.X (Math|Vector2D|BreakVector2D (.ScreenLocation (Class|PlayerController|ProjectWorldLocationtoScreen (Game|GetPlayerController 0) (Transformation|GetActorLocation _array_element) true)))) _x_4) (< (.Y (Math|Vector2D|BreakVector2D (.ScreenLocation (Class|PlayerController|ProjectWorldLocationtoScreen (Game|GetPlayerController 0) (Transformation|GetActorLocation _array_element) true)))) _y_4))
      (if (not (stale _output_get))
        ;[1 1 1] feels too jumpy
        (Variables|Default|SetSomeoneOffScreen false))
      (else
        (bind _output_get (Variables|Default|SetSomeoneOffScreen true)))))
  (Transformation|SetActorRotation (Math|Rotator|FindLookatRotation _returnvalue_6 _returnvalue_5))
  (Transformation|SetActorLocation _self (Math|Vector|MakeVector (- (/ (.X (Math|Vector|BreakVector _returnvalue_5)) 8.0) 2e+02) 1.7e+03 (.Z (Math|Vector|BreakVector _returnvalue_6))) false false)
  (if (Variables|Default|GetSomeoneOffScreen)
    (Transformation|SetActorLocation (Math|Vector|MakeVector _x_3 _y_3 (+ _z_2 (Variables|Default|GetHeightMultiplier))) true false)
    (for _array_element_2 (Variables|Default|GetActivePlayers)
      (if (Math|Boolean|ANDBoolean (> (.X (Math|Vector2D|BreakVector2D (.ScreenLocation (Class|PlayerController|ProjectWorldLocationtoScreen (Game|GetPlayerController 0) (Transformation|GetActorLocation _array_element_2) true)))) 0.0) (> (.Y (Math|Vector2D|BreakVector2D (.ScreenLocation (Class|PlayerController|ProjectWorldLocationtoScreen (Game|GetPlayerController 0) (Transformation|GetActorLocation _array_element_2) true)))) 0.0) (< (.X (Math|Vector2D|BreakVector2D (.ScreenLocation (Class|PlayerController|ProjectWorldLocationtoScreen (Game|GetPlayerController 0) (Transformation|GetActorLocation _array_element_2) true)))) _x) (< (.Y (Math|Vector2D|BreakVector2D (.ScreenLocation (Class|PlayerController|ProjectWorldLocationtoScreen (Game|GetPlayerController 0) (Transformation|GetActorLocation _array_element_2) true)))) _y))
        (if (not (stale _output_get_2))
          (Variables|Default|SetKeepZooming false))
        (else
          (bind _output_get_2 (Variables|Default|SetKeepZooming true)))))
    (if (and (Variables|Default|GetSomeoneOffScreen) (Variables|Default|GetKeepZooming))
      (Variables|Default|SetHeightMultiplier (Math|Float|Max(Float) (* (Variables|Default|GetHeightMultiplier) 1.1) 0.5))
      (Variables|Default|SetKeepZooming false)
      (else
        (Variables|Default|SetHeightMultiplier 0.1)
        (Variables|Default|SetSomeoneOffScreen false)))
    (elif (> (- _z (Variables|Default|GetHeightMultiplier)) 1.5e+03)
      (Transformation|SetActorLocation (Math|Vector|MakeVector _x_2 _y_2 (- _z (Variables|Default|GetHeightMultiplier))) true false)
      (Variables|Default|SetSomeoneOffScreen false)
      (Variables|Default|SetKeepZooming false)
      (Variables|Default|SetHeightMultiplier (Math|Float|Max(Float) (* (Variables|Default|GetHeightMultiplier) 1.05) 0.5))
      (else
        (Variables|Default|SetHeightMultiplier 0.1)
        (Variables|Default|SetSomeoneOffScreen false)
        (Variables|Default|SetKeepZooming false)))))

(fn ConstructionScript)